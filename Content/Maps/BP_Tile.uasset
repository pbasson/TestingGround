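; BP_Tile is a level segment for an infinite game that scatters containers, boxes and canisters via PlaceActors on BeginPlay.
; Its barrier starts locked, turns green and passable while the player overlaps BoxVolume, then relocks on exit as InfiniteGameMode spawns another tile.
; The tile destroys itself when the player enters NextVolume.
; An Arrow component's world transform is exposed as the attachment point.
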(event `self.ReceiveBeginPlay`
  (`self.Lock`)
  (`self.PlaceActors` "/Game/Maps/Map_Elements/BP_Container.BP_Container_C" 0 3)
  (`self.PlaceActors` "/Game/Maps/Map_Elements/BP_Box.BP_Box_C" 2 4 500.0 1.0 5.0)
  (`self.PlaceActors` "/Game/Maps/Map_Elements/BP_Canister.BP_Canister_C" 2 4 500.0 1.0 2.0))

(event `self.BoxVolume.OnComponentBeginOverlap`
  (params (OverlappedComponent :type "PrimitiveComponent Object Reference") (OtherActor :type "Actor Object Reference") (OtherComp :type "PrimitiveComponent Object Reference") (OtherBodyIndex :type Integer) (bFromSweep :type Boolean) (SweepResult :type "HitResult Structure (by ref)"))
  (`self.IsPlayer` OtherActor
    (:`OutPut`
      (`self.Unlock`))))

(event `self.BoxVolume.OnComponentEndOverlap`
  (params (OverlappedComponent :type "PrimitiveComponent Object Reference") (OtherActor :type "Actor Object Reference") (OtherComp :type "PrimitiveComponent Object Reference") (OtherBodyIndex :type Integer))
  (`self.IsPlayer` OtherActor
    (:`OutPut`
      (`self.Lock`)
      (bind _asinfinite_game_mode (cast `/Game/Blueprints/InfiniteGameMode` (`GameplayStatics.GetGameMode`)))
      (`/Game/Blueprints/InfiniteGameMode.SpawnTile` _asinfinite_game_mode))))

(event `self.NextVolume.OnComponentBeginOverlap`
  (params (OverlappedComponent :type "PrimitiveComponent Object Reference") (OtherActor :type "Actor Object Reference") (OtherComp :type "PrimitiveComponent Object Reference") (OtherBodyIndex :type Integer) (bFromSweep :type Boolean) (SweepResult :type "HitResult Structure (by ref)"))
  (`self.IsPlayer` OtherActor
    (:`OutPut`
      (`self.K2_DestroyActor`))))

(fn `GetAttachedLocation`
  (returns (AttachTransform :type "Transform Structure"))
  (return (`SceneComponent.K2_GetComponentToWorld` (`self.Arrow`))))

(fn `Lock`
  (bind _barrier (`self.Barrier`))
  (`PrimitiveComponent.SetCollisionEnabled` _barrier "QueryAndPhysics")
  (`PrimitiveComponent.SetMaterial` _barrier 0 "/Game/Geometry/Meshes/Red_Barrier.Red_Barrier"))

(fn `Unlock`
  (bind _barrier (`self.Barrier`))
  (`PrimitiveComponent.SetCollisionEnabled` _barrier "NoCollision")
  (`PrimitiveComponent.SetMaterial` _barrier 0 "/Game/Geometry/Meshes/Green_Barrier.Green_Barrier"))

(fn `UserConstructionScript`)