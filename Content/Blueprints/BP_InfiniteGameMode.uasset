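; BP_InfiniteGameMode is a game mode that builds a chain of tiles and keeps score of completed ones.
; On BeginPlay it populates a pool of nav mesh bounds volumes, then spawns a few initial tiles.
; SpawnTile hands each new BP_Tile that shared pool and takes its attach location as the next spawn transform, laying tiles end to end.
; CompletedTile increments the score.
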(event `self.ReceiveBeginPlay`
  (`self.PopulateBoundsVolumePool`)
  (for _ (range 3)
    (`self.SpawnTile`)))

(fn `CompletedTile`
  (`/Engine/EditorBlueprintResources/StandardMacros.IncrementInt` (`self.Score`)))

(fn `SpawnTile`
  (bind _returnvalue (`|SpawnActorFromClass` "/Game/Maps/BP_Tile.BP_Tile_C" (`self.NextTilePos`) "Undefined" "OverrideRootScale" null null))
  (`Tile.SetPool` _returnvalue (`self.NavMeshBoundsVolumePool`))
  (bind _attachtransform (`/Game/Maps/BP_Tile.GetAttachedLocation` _returnvalue))
  (set `self.NextTilePos` _attachtransform))

(fn `UserConstructionScript`)