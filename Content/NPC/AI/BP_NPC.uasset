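; BP_NPC is an NPC AI controller that runs a patrol behavior tree and tracks sensed actors as enemies.
; On BeginPlay it initializes the PatrolData blackboard, starts the Patrol tree and caches the blackboard component.
; AI perception updates write sensed actors without the "Enemy" tag to EnemyKey and clear the key when such an actor is lost.
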(event `self.ReceiveBeginPlay`
  ;[1 1 1] BeginPlay
  (bind _blackboardcomponent (`self.UseBlackboard` "/Game/NPC/AI/BehaviourTree/PatrolData.PatrolData"))
  (`self.RunBehaviorTree` "/Game/NPC/AI/BehaviourTree/Patrol.Patrol")
  (set `self.BlackboardComp` _blackboardcomponent))

(event `self.AIPerception.OnTargetPerceptionUpdated`
  (params (Actor :type "Actor Object Reference") (Stimulus :type "AIStimulus Structure"))
  (bind _enemykey (`self.EnemyKey`))
  (bind _blackboardcomp (`self.BlackboardComp`))
  ;[1 1 1] OnTargetPerception
  (if (`self.ActorHasTag` Actor "Enemy")
    _
    (elif (`.bSuccessfullySensed` (break `AIStimulus` Stimulus))
      (`BlackboardComponent.SetValueAsObject` _blackboardcomp _enemykey Actor)
      (else
        (`BlackboardComponent.ClearValue` _blackboardcomp _enemykey)))))

(event `self.ReceiveTick`
  (params (DeltaSeconds :type "Float (single-precision)"))
  ;[1 1 1] Tick
)

(fn `UserConstructionScript`)