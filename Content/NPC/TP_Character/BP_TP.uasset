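; BP_TP is a third-person character in the NPC folder with axis-driven movement and a health widget.
; MoveForward and MoveRight add movement along directions derived from control yaw only, ignoring pitch and roll.
; On BeginPlay, HealthFunctionSetup casts the MannequinWidget's user widget to Health_UI and passes it a reference to this character.
; IsDead reports whether current health is at or below zero.
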(event `InputAxis|MoveForward`
  (params (AxisValue :type "Float (single-precision)"))
  ;[1 1 1] Movement_Input
  (`self.AddMovementInput` (`KismetMathLibrary.GetForwardVector` (`KismetMathLibrary.MakeRotator` 0.0 0.0 (.yaw (`self.GetControlRotation`)))) AxisValue))

(event `InputAxis|MoveRight`
  (params (AxisValue :type "Float (single-precision)"))
  ;[1 1 1] Movement_Input
  (`self.AddMovementInput` (`KismetMathLibrary.GetRightVector` (`KismetMathLibrary.MakeRotator` 0.0 0.0 (.yaw (`self.GetControlRotation`)))) AxisValue))

(event `self.ReceiveBeginPlay`
  (`self.HealthFunctionSetup`))

(fn `HealthFunctionSetup`
  (bind _ashealth_ui (cast `/Game/UI/Health_UI` (`WidgetComponent.GetUserWidgetObject` (`self.MannequinWidget`))))
  (set `/Game/UI/Health_UI.Mannequin` self _ashealth_ui))

(fn `IsDead`
  (returns (Dead :type Boolean))
  (return (<= (`self.HealthCurrent`) 0.0)))

(fn `UserConstructionScript`)